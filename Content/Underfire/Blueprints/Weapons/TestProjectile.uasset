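; Test bullet projectile that draws speed-coloured debug traces and prototypes material penetration.
; On bounce it spawns an impact actor, then fast hits seek an exit point to respawn the projectile with unchanged impact velocity, destroying the original.
; CalculateExitLocation sphere-traces backwards through the hit actor, recursing through adjoining objects.
; The GetNewSpeed check gates respawning, but its kinetic-energy loss formula is unwired.
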(event `self.ReceiveTick`
  (params (DeltaSeconds :type "Float (single-precision)"))
  (bind _returnvalue (`self.K2_GetActorLocation`))
  (bind _color (`self.Get Trace Color` (`MovementComponent.Velocity` (`self.ProjectileMovement`))))
  (`KismetSystemLibrary.DrawDebugLine` (`self.Last Position`) _returnvalue _color (`self.Trace Duration`))
  (set `self.Last Position` _returnvalue))

(event `self.ProjectileMovement.OnProjectileBounce`
  (params (ImpactResult :type "HitResult Structure (by ref)") (ImpactVelocity :type "Vector Structure (by ref)"))
  (bind (_bblockinghit _binitialoverlap _time _location) (`GameplayStatics.BreakHitResult` ImpactResult))
  (bind _last_position (`self.Last Position`))
  (`|SpawnActorFromClass` "/Game/Underfire/Blueprints/Bullet_Impacts/Bullet_Impact_Test_No_Decal.Bullet_Impact_Test_No_Decal_C" (`KismetMathLibrary.MakeTransform` _location (`KismetMathLibrary.FindLookAtRotation` _location _last_position)) "Undefined" "OverrideRootScale")
  (bind _color (`self.Get Trace Color` ImpactVelocity))
  (`KismetSystemLibrary.DrawDebugLine` _last_position _location _color (`self.Trace Duration`))
  (set `self.Last Position` _location)
  (if (> (`KismetMathLibrary.VSize` ImpactVelocity) (`self.Speed to penetrate`))
    (bind (_exit_location _exit_normal _result_found) (`self.Calculate Exit Location` ImpactResult ImpactVelocity))
    (if (> (`self.Get New Speed` ImpactResult _exit_normal ImpactVelocity) 0.0)
      (if _result_found
        (bind _returnvalue (`|SpawnActorFromClass` "TestProjectile_C" (`KismetMathLibrary.MakeTransform` _exit_location) "Undefined" "OverrideRootScale" (`self.GetOwner`)))
        (set `MovementComponent.Velocity` ImpactVelocity (`UnderFireProjectile.ProjectileMovement` _returnvalue))
        (`self.K2_DestroyActor`)
        (else
          (`self.K2_DestroyActor`)))
      (else
        ;[1 1 1] Projectile moved to slow to exit material
        (`self.K2_DestroyActor`)))
    (else
      (`self.K2_DestroyActor`))))

(event `self.CollisionComp.OnComponentBeginOverlap`
  (params (OverlappedComponent :type "PrimitiveComponent Object Reference") (OtherActor :type "Actor Object Reference") (OtherComp :type "PrimitiveComponent Object Reference") (OtherBodyIndex :type Integer) (bFromSweep :type Boolean) (SweepResult :type "HitResult Structure (by ref)"))
  (`KismetSystemLibrary.PrintString` "overlap has begun"))

(fn `Calculate Exit Location`
  (params (`Hit Results` :type "HitResult Structure") (`Impact Velocity` :type "Vector Structure"))
  (returns (`Exit Location` :type "Vector Structure") (`Exit Normal` :type "Vector Structure") (`Result Found` :type Boolean))
  (bind (_bblockinghit _binitialoverlap _time _location _impactpoint _normal _impactnormal _physmat _hitactor) (`GameplayStatics.BreakHitResult` `Hit Results`))
  (bind _returnvalue (`KismetMathLibrary.Normal` `Impact Velocity`))
  (bind _array (`|MakeArray` "ObjectTypeQuery1" "ObjectTypeQuery2" "ObjectTypeQuery3" "ObjectTypeQuery4" "ObjectTypeQuery6" :!type "EObjectTypeQuery Enum"))
  (bind (_outhits _returnvalue_2) (`KismetSystemLibrary.SphereTraceMultiForObjects` (+ _location (* _returnvalue 500.0)) _location (`SphereComponent.SphereRadius` (`self.CollisionComp`)) _array))
  (if _returnvalue_2
    (for (_ _array_index) _outhits
      (bind (_bblockinghit_2 _binitialoverlap_2 _time_2 _location_2 _impactpoint_2 _normal_2 _impactnormal_2 _physmat_2 _hitactor_2) (`GameplayStatics.BreakHitResult` (`KismetArrayLibrary.Array_Get` _outhits (- (`KismetArrayLibrary.Array_LastIndex` _outhits) _array_index))))
      (if (== _hitactor_2 _hitactor)
        (bind _returnvalue_3 (+ _location_2 _impactnormal_2))
        (bind (_outhit _returnvalue_4) (`KismetSystemLibrary.SphereTraceSingleForObjects` _returnvalue_3 (+ _returnvalue_3 _returnvalue) (`SphereComponent.SphereRadius` (`self.CollisionComp`)) _array false (`|MakeArray` _hitactor)))
        (if _returnvalue_4
          (bind (_exit_location _exit_normal _result_found) (`self.Calculate Exit Location` _outhit `Impact Velocity`))
          (return _exit_location _exit_normal _result_found)
          (else
            (return _returnvalue_3 _impactnormal_2 true))))))
  (return (0.0 0.0 0.0) (0.0 0.0 0.0) false))

(fn `Get Trace Color`
  (params (Velocity :type "Vector Structure"))
  (returns (Color :type "LinearColor Structure"))
  (bind _returnvalue (/ (`KismetMathLibrary.VSize` Velocity) (`ProjectileMovementComponent.MaxSpeed` (`self.ProjectileMovement`))))
  (bind _returnvalue_2 (- _returnvalue 0.25))
  (if (> _returnvalue 0.75)
    (return (`KismetMathLibrary.LinearColorLerp` (struct :`B` 1.0 :`A` 1.0) (struct :`G` 1.0 :`A` 1.0) (* (- _returnvalue 0.75) 4.0)))
    (elif (> _returnvalue 0.5)
      (return (`KismetMathLibrary.LinearColorLerp` (struct :`B` 1.0 :`A` 1.0) (struct :`R` 1.0 :`G` 1.0 :`A` 1.0) (- _returnvalue 0.5)))
      (elif (> _returnvalue 0.25)
        (return (`KismetMathLibrary.LinearColorLerp` (struct :`R` 1.0 :`G` 1.0 :`A` 1.0) (struct :`R` 1.0 :`A` 1.0) _returnvalue_2))
        (else
          (return (`KismetMathLibrary.LinearColorLerp` (struct :`R` 1.0 :`A` 1.0) (struct :`A` 1.0) _returnvalue_2)))))))

(fn `UserConstructionScript`
  (set `self.Last Position` (`self.K2_GetActorLocation`)))