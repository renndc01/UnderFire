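; Instant-type weapon Blueprint that handles the cosmetic firing effects, with no hit or damage logic in its graphs.
; FireEvent spawns the muzzle flash and shell ejection emitters at their named sockets on the weapon mesh.
; Both go through a shared SpawnEffect helper, which skips unset effects and attaches each emitter at the socket's world transform using KeepWorldPosition.
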(event `self.Fire_Event`
  (`self.Spawn Effect` (`self.Muzzle Flash Effect`) (`self.Name of Muzzle Socket`))
  (`self.Spawn Effect` (`self.Shell Eject Effect`) (`self.Name of Shell Ejection Socket`)))

(fn `Spawn Effect`
  (params (Effect :type "ParticleSystem Object Reference") (`Socket Name` :type Name))
  (bind _weaponmesh (`self.WeaponMesh`))
  (bind (_returnvalue_location _returnvalue_rotation) (`KismetMathLibrary.BreakTransform` (`SceneComponent.GetSocketTransform` _weaponmesh `Socket Name` "RTS_World")))
  (`/Engine/EditorBlueprintResources/StandardMacros.IsValid` Effect
    (:`Is Valid`
      (`GameplayStatics.SpawnEmitterAttached` Effect _weaponmesh `Socket Name` _returnvalue_location _returnvalue_rotation "KeepWorldPosition"))))

(fn `UserConstructionScript`)