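; Tutorial level game mode that steps through shooting range stages by toggling groups of ShootingTarget actors.
; UpdateShootingRange flips IsActive and calls CycleLight on targets whose OrderCount matches CurrentRange, increments CurrentRange, then does the same for the next group.
; BeginPlay runs this update once; no other call to it appears in this Blueprint.
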(event `self.ReceiveBeginPlay`
  (`self.Update Shooting Range`))

(fn `Update Shooting Range`
  (bind _outactors (`GameplayStatics.GetAllActorsOfClass` "/Game/Underfire/Blueprints/Shooting_Range/ShootingTarget.ShootingTarget_C"))
  (for _array_element _outactors
    (if (== (`/Game/Underfire/Blueprints/Shooting_Range/ShootingTarget.Order Count` _array_element) (`self.Current Range`))
      (set `/Game/Underfire/Blueprints/Shooting_Range/ShootingTarget.Is active` (not (`/Game/Underfire/Blueprints/Shooting_Range/ShootingTarget.Is active` _array_element)) _array_element)
      (`/Game/Underfire/Blueprints/Shooting_Range/ShootingTarget.Cycle Light` _array_element)))
  (bind _result (`/Engine/EditorBlueprintResources/StandardMacros.IncrementInt` (`self.Current Range`))
    (:`  `
      (bind _outactors_2 (`GameplayStatics.GetAllActorsOfClass` "/Game/Underfire/Blueprints/Shooting_Range/ShootingTarget.ShootingTarget_C"))
      (for _array_element_2 _outactors_2
        (if (== (`/Game/Underfire/Blueprints/Shooting_Range/ShootingTarget.Order Count` _array_element_2) _result)
          (set `/Game/Underfire/Blueprints/Shooting_Range/ShootingTarget.Is active` (not (`/Game/Underfire/Blueprints/Shooting_Range/ShootingTarget.Is active` _array_element_2)) _array_element_2)
          (`/Game/Underfire/Blueprints/Shooting_Range/ShootingTarget.Cycle Light` _array_element_2))))))

(fn `UserConstructionScript`)