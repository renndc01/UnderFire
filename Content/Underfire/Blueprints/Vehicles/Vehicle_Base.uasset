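; Base vehicle Blueprint that plays engine or movement sounds based on the CurrentMovement state.
; BeginPlay and Tick call SelectVehicleSound, which picks idle, fast or slow sounds, shared between forward and reverse.
; SetNewVehicleSound plays a one-shot at the actor's location, leaving the VehicleSound component swap unconnected.
; PreviousMovement is only stored at BeginPlay, so Tick retriggers the sound every frame while the state differs from that initial value.
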(event `self.ReceiveBeginPlay`
  (set `self.Previous Movement` (`self.Current Movement`))
  (`self.Select Vehicle Sound`))

(event `self.ReceiveTick`
  (params (DeltaSeconds :type "Float (single-precision)"))
  (if (!= (`self.Current Movement`) (`self.Previous Movement`))
    (`self.Select Vehicle Sound`)))

(fn `Select Vehicle Sound`
  (switch `/Game/Underfire/Blueprints/Vehicles/Vehicle_Movement` (`self.Current Movement`)
    (:`NewEnumerator0`
      (`self.Set New Vehicle Sound` (`self.Idle Sound`)))
    (:`NewEnumerator1`
      (`self.Set New Vehicle Sound` (`self.Move Fast Sound`) :!label _label))
    (:`NewEnumerator2`
      (`self.Set New Vehicle Sound` (`self.Move Slow Sound`) :!label _label_2))
    (:`NewEnumerator3`
      (goto _label))
    (:`NewEnumerator4`
      (goto _label_2))))

(fn `Set New Vehicle Sound`
  (params (`New Sound` :type "SoundBase Object Reference"))
  (`GameplayStatics.PlaySoundAtLocation` `New Sound` (`self.K2_GetActorLocation`)))

(fn `UserConstructionScript`)