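; Tutorial shooting range target with a child LightPole, active while the player stands in its start box and the game mode allows range changes.
; Overlap toggles the pole's visibility.
; Tick polls the player's action button and distance to change the light's color once until the player exits.
; Five hits while active, or a 0.6 shot average on reload from empty, advances the range through Level_Tutorial_GameMode.
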(event `self.ReceiveBeginPlay`
  (`self.Cycle Light`))

(event `self.ReceiveTick`
  (params (DeltaSeconds :type "Float (single-precision)"))
  (bind _outactors (`GameplayStatics.GetAllActorsOfClass` "/Game/Underfire/Blueprints/Characters/UnderfirePlayerCharacterBP.UnderfirePlayerCharacterBP_C"))
  (bind _item (`KismetArrayLibrary.Array_Get` _outactors))
  (bind _returnvalue (and (`UnderFirePlayerCharacter.isActionButtonPressed` _item) (<= (`KismetMathLibrary.VSize` (- (`SceneComponent.K2_GetComponentLocation` (`self.Start Target Shoot Collision`)) (`self.K2_GetActorLocation` _item))) 250.0) (`self.Can Change light`)))
  (`KismetSystemLibrary.PrintString` (`KismetStringLibrary.Conv_BoolToString` _returnvalue) true true (struct :`G` 0.66 :`B` 1.0 :`A` 1.0) 0.0)
  (if _returnvalue
    (`self.Change Light Color`)
    (set `self.Can Change light` false)))

(event `self.Start Target Shoot Collision.OnComponentBeginOverlap`
  (params (OverlappedComponent :type "PrimitiveComponent Object Reference") (OtherActor :type "Actor Object Reference") (OtherComp :type "PrimitiveComponent Object Reference") (OtherBodyIndex :type Integer) (bFromSweep :type Boolean) (SweepResult :type "HitResult Structure (by ref)"))
  (bind _asunder_fire_player_character (cast `UnderFirePlayerCharacter` OtherActor))
  (set `self.Player is In Start Box` true)
  (`self.Check for Light Color Change` _asunder_fire_player_character)
  (bind _aslevel_tutorial_game_mode (cast `/Game/Underfire/Blueprints/Level_Tutorial_GameMode` (`GameplayStatics.GetGameMode`)))
  (if (`/Game/Underfire/Blueprints/Level_Tutorial_GameMode.Can Change Range` _aslevel_tutorial_game_mode)
    (if (not (`self.Is active`))
      (set `self.Player is in Shooting Range` true)
      (set `self.Is active` true)
      (`self.Cycle Light`))))

(event `self.Start Target Shoot Collision.OnComponentEndOverlap`
  (params (OverlappedComponent :type "PrimitiveComponent Object Reference") (OtherActor :type "Actor Object Reference") (OtherComp :type "PrimitiveComponent Object Reference") (OtherBodyIndex :type Integer))
  (cast `UnderFirePlayerCharacter` OtherActor)
  (set `self.Can Change light` true)
  (set `self.Player is in Shooting Range` false)
  (bind _aslevel_tutorial_game_mode (cast `/Game/Underfire/Blueprints/Level_Tutorial_GameMode` (`GameplayStatics.GetGameMode`)))
  (if (`/Game/Underfire/Blueprints/Level_Tutorial_GameMode.Can Change Range` _aslevel_tutorial_game_mode)
    (if (`self.Is active`)
      (set `self.Player is in Shooting Range` false)
      (set `self.Is active` false)
      (`self.Cycle Light`))))

(event `Reload From Empty Event`
  (if (>= (`self.Shot Average`) 0.6)
    (bind _aslevel_tutorial_game_mode (cast `/Game/Underfire/Blueprints/Level_Tutorial_GameMode` (`GameplayStatics.GetGameMode`)))
    (`/Game/Underfire/Blueprints/Level_Tutorial_GameMode.Update Shooting Range` _aslevel_tutorial_game_mode)))

(event `Hit Target Event`
  (if (`self.Is active`)
    (bind _result (`/Engine/EditorBlueprintResources/StandardMacros.IncrementInt` (`self.Shot Hit Count`))
      (:`  `
        (if (>= _result 5)
          (bind _aslevel_tutorial_game_mode (cast `/Game/Underfire/Blueprints/Level_Tutorial_GameMode` (`GameplayStatics.GetGameMode`)))
          (`/Game/Underfire/Blueprints/Level_Tutorial_GameMode.Update Shooting Range` _aslevel_tutorial_game_mode))))))

(event `self.StaticMesh6.OnComponentHit`
  (params (HitComponent :type "PrimitiveComponent Object Reference") (OtherActor :type "Actor Object Reference") (OtherComp :type "PrimitiveComponent Object Reference") (NormalImpulse :type "Vector Structure") (Hit :type "HitResult Structure (by ref)"))
  (`KismetSystemLibrary.PrintString` "Hit Target"))

(fn `Calculate Shot Average`
  (set `self.Shot Average` (`KismetMathLibrary.Conv_IntToDouble` (/ (`self.Shot Hit Count`) (`self.Shot Count`)))))

(fn `Change Light Color`
  (bind _aslight_pole (cast `/Game/Underfire/Blueprints/Shooting_Range/LightPole` (`ChildActorComponent.ChildActor` (`self.LightPole`))))
  (`/Game/Underfire/Blueprints/Shooting_Range/LightPole.Change Color` _aslight_pole))

(fn `Check for Light Color Change`
  (params (Player :type "UnderFirePlayerCharacter Object Reference")))

(fn `Cycle Light`
  (bind _aslight_pole (cast `/Game/Underfire/Blueprints/Shooting_Range/LightPole` (`ChildActorComponent.ChildActor` (`self.LightPole`))))
  (`/Game/Underfire/Blueprints/Shooting_Range/LightPole.Cycle Visiblity` _aslight_pole))

(fn `Increase Shot Count`
  (`/Engine/EditorBlueprintResources/StandardMacros.IncrementInt` (`self.Shot Count`)))

(fn `UserConstructionScript`)