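; Shooting range light pole with a spotlight and a light shaft mesh that can be toggled or recolored.
; Construction applies the start intensity and normal color, while Tick pushes CurrentColor to both the light and the shaft material every frame.
; CycleVisiblity flips spotlight visibility.
; ChangeColor re-rolls a random number at each branch, so red, green, blue and normal are unevenly weighted and the color can stay unchanged.
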(event `self.ReceiveBeginPlay`
  (set `self.Current Color` (`self.Normal Color`)))

(event `self.ReceiveTick`
  (params (DeltaSeconds :type "Float (single-precision)"))
  (bind _current_color (`self.Current Color`))
  (`LightComponent.SetLightColor` (`self.SpotLight`) (`KismetMathLibrary.Conv_VectorToLinearColor` _current_color) true)
  (`MeshComponent.SetVectorParameterValueOnMaterials` (`self.Light Ray`) "Light Shaft Color" _current_color))

(fn `Change Color`
  (bind _returnvalue (`KismetMathLibrary.RandomIntegerInRange` 1 4))
  (if (== _returnvalue 1)
    (set `self.Current Color` (`self.Red Color`))
    (elif (== _returnvalue 2)
      (set `self.Current Color` (`self.Green Color`))
      (elif (== _returnvalue 3)
        (set `self.Current Color` (`self.Blue Color`))
        (elif (>= _returnvalue 4)
          (set `self.Current Color` (`self.Normal Color`)))))))

(fn `Cycle Visiblity`
  (bind _spotlight (`self.SpotLight`))
  (`SceneComponent.SetVisibility` _spotlight (not (`SceneComponent.bVisible` _spotlight)) true))

(fn `UserConstructionScript`
  (bind _spotlight (`self.SpotLight`))
  (bind _normal_color (`self.Normal Color`))
  (`LightComponent.SetIntensity` _spotlight (`self.Start Intensity`))
  (`LightComponent.SetLightColor` _spotlight (`KismetMathLibrary.Conv_VectorToLinearColor` _normal_color) true)
  (`MeshComponent.SetVectorParameterValueOnMaterials` (`self.Light Ray`) "Light Shaft Color" _normal_color))