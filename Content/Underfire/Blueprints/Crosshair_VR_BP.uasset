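; Crosshair actor for VR that floats in the world ahead of the owning character's current weapon.
; Each Tick, while the owning character is valid, it moves to a point projected far along the weapon mesh's right vector, with small forward and up offsets.
; It then uses a look-at rotation to face the character's first-person camera.
; Placement is purely offset-based, with no trace against the scene.
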(event `self.ReceiveTick`
  (params (DeltaSeconds :type "Float (single-precision)"))
  (bind _owning_character (`self.Owning Character`))
  (bind _weaponmesh (`UFWeapon.WeaponMesh` (`UnderFireCharacter.currentWeapon` _owning_character)))
  (bind _returnvalue (+ (* (`SceneComponent.GetUpVector` _weaponmesh) 25) (+ (* (`SceneComponent.GetForwardVector` _weaponmesh) 25) (+ (`SceneComponent.K2_GetComponentLocation` _weaponmesh) (* (`SceneComponent.GetRightVector` _weaponmesh) 1000)))))
  (`/Engine/EditorBlueprintResources/StandardMacros.IsValid` _owning_character
    (:`Is Valid`
      (`self.K2_SetActorLocation` _returnvalue)
      (`self.K2_SetActorRotation` (`KismetMathLibrary.FindLookAtRotation` _returnvalue (`SceneComponent.K2_GetComponentLocation` (`UnderFirePlayerCharacter.FirstPersonCameraComponent` _owning_character)))))))

(fn `UserConstructionScript`)