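; Underfire AI character Blueprint that fades out the body after death.
; While IsDead is set, Tick calls BodyFadeOut, which uses the JustDied flag to swap mesh material slot 0 to a translucent dynamic instance once.
; Later frames lower its "Tranparency" (sic) parameter linearly from one to zero over a minute, printing the value on screen.
; The value is not clamped and the actor is never destroyed here.
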(event `self.ReceiveActorBeginOverlap`
  (params (OtherActor :type "Actor Object Reference")))

(event `self.ReceiveTick`
  (params (DeltaSeconds :type "Float (single-precision)"))
  (if (`self.isDead`)
    (`self.Body Fade Out`)))

(fn `Body Fade Out`
  (bind _item (`KismetArrayLibrary.Array_Get` (`MeshComponent.GetMaterials` (`self.Mesh`))))
  (if (`self.Just Died`)
    (bind _returnvalue (`KismetMaterialLibrary.CreateDynamicMaterialInstance` _item "/Game/Underfire/Character/Materials/M_UE4Man_Body_Translucent.M_UE4Man_Body_Translucent"))
    (`PrimitiveComponent.SetMaterial` (`self.Mesh`) 0 _returnvalue)
    (set `self.Just Died` false)
    (else
      (bind _asmaterial_instance_dynamic (cast `MaterialInstanceDynamic` _item))
      (bind _output_get (set `self.Total Body Time` (+ (`GameplayStatics.GetWorldDeltaSeconds`) (`self.Total Body Time`))))
      (bind _returnvalue_2 (/ (- 60.0 _output_get) 60.0))
      (`MaterialInstanceDynamic.SetScalarParameterValue` _asmaterial_instance_dynamic "Tranparency" _returnvalue_2)
      (`KismetSystemLibrary.PrintString` (`KismetStringLibrary.Conv_DoubleToString` _returnvalue_2) true true (struct :`G` 0.66 :`B` 1.0 :`A` 1.0) 0.0))))

(fn `UserConstructionScript`)