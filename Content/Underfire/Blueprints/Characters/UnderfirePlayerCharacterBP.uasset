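; Player character Blueprint for Underfire, handling first-person view, crosshair and HUD setup for VR and flat-screen play.
; BeginPlay spawns an owned crosshair actor when a headset is enabled, otherwise adds crosshair and HUD widgets to the viewport.
; Tick prints weapon, ammo, health and death debug text and copies headset rotation to the camera.
; DeathEvent attempts an interpolated camera turn along the mesh-to-camera direction, but its zero delta time prevents movement.
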(event `self.ReceiveBeginPlay`
  (if (`HeadMountedDisplayFunctionLibrary.IsHeadMountedDisplayEnabled`)
    (bind _returnvalue (`|SpawnActorFromClass` "/Game/Underfire/Blueprints/Crosshair_VR_BP.Crosshair_VR_BP_C" (`KismetMathLibrary.MakeTransform` (0.0 0.0 0.0)) "Undefined" "OverrideRootScale"))
    (set `/Game/Underfire/Blueprints/Crosshair_VR_BP.Owning Character` self _returnvalue)
    (else
      (bind _returnvalue_2 (`|CreateWidget` (`self.CrossHair Class`)))
      (bind _output_get (set `self.CrossHair` _returnvalue_2))
      (`UserWidget.AddToViewport` _output_get 0)
      (bind _returnvalue_3 (`|CreateWidget` "/Game/Underfire/Blueprints/HUD.HUD_C"))
      (bind _output_get_2 (set `self.HUD` _returnvalue_3))
      (`UserWidget.AddToViewport` _output_get_2 0))))

(event `self.ReceiveTick`
  (params (DeltaSeconds :type "Float (single-precision)"))
  (bind _currentweapon (`self.currentWeapon`))
  (`KismetSystemLibrary.PrintString` (`KismetStringLibrary.Conv_NameToString` (`UFWeapon.WeaponName` _currentweapon)) true false (struct :`R` 1.0 :`B` 0.723107 :`A` 1.0) 0.0)
  (`KismetSystemLibrary.PrintString` (`KismetStringLibrary.Conv_IntToString` (`UFWeapon.ClipCurrentAmmo` _currentweapon)) true false (struct :`R` 1.0 :`B` 0.723107 :`A` 1.0) 0.0)
  (`KismetSystemLibrary.PrintString` (`KismetStringLibrary.Conv_IntToString` (`UFWeapon.StockCurrentAmmo` _currentweapon)) true false (struct :`R` 1.0 :`B` 0.723107 :`A` 1.0) 0.0)
  (`KismetSystemLibrary.PrintString` (`KismetStringLibrary.Conv_DoubleToString` (`self.CurrentHealth`)) true false (struct :`R` 1.0 :`G` 0.016322 :`A` 1.0) 0.0)
  (`KismetSystemLibrary.PrintString` (`KismetStringLibrary.Conv_BoolToString` (`self.isDead`)) true false (struct :`G` 0.66 :`B` 1.0 :`A` 1.0) 0.0)
  (`SceneComponent.K2_SetRelativeRotation` (`self.FirstPersonCameraComponent`) (`HeadMountedDisplayFunctionLibrary.GetOrientationAndPosition`) false false))

(event `self.Death_Event`
  (bind _firstpersoncameracomponent (`self.FirstPersonCameraComponent`))
  (`KismetSystemLibrary.PrintString` "Death Event")
  (`SceneComponent.K2_SetWorldRotation` _firstpersoncameracomponent (`KismetMathLibrary.RInterpTo` (`SceneComponent.K2_GetComponentRotation` _firstpersoncameracomponent) (`KismetMathLibrary.FindLookAtRotation` (`SceneComponent.K2_GetComponentLocation` (`self.Mesh`)) (`SceneComponent.K2_GetComponentLocation` _firstpersoncameracomponent)) 0.0 5.0) false false))

(fn `UserConstructionScript`)