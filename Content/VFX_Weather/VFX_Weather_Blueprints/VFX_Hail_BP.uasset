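; Hail weather effect actor that exposes color, spawn rate and forces for its particle component.
; HailParameters writes these values to the particle system's parameters, randomly scaling each force axis on every call for variation.
; It runs from the construction script and again every Tick, so forces fluctuate continuously during play.
; The construction script and BeginPlay also store a dynamic instance of the hail material, which the graphs never modify.
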(event `self.ReceiveBeginPlay`
  (bind _returnvalue (`PrimitiveComponent.CreateDynamicMaterialInstance` (`self.VFX_Weather_Hail_ForBP`) 0 "/Game/VFX_Weather/VFX_Weather_Materials/Hail_Inst.Hail_Inst"))
  (set `self.HailMat` _returnvalue))

(event `self.ReceiveTick`
  (params (DeltaSeconds :type "Float (single-precision)"))
  (`self.HailParameters`))

(fn `HailParameters`
  (bind _returnvalue (`KismetMathLibrary.RandomFloatInRange` 0.5 1.5))
  (`ParticleSystemComponent.SetVectorParameter` (`self.VFX_Weather_Hail_ForBP`) "HailColor" (`KismetMathLibrary.Conv_LinearColorToVector` (`self.HailColor`)))
  (`ParticleSystemComponent.SetFloatParameter` (`self.VFX_Weather_Hail_ForBP`) "DetailHailSpawn" (`self.SpawnRate`))
  (`ParticleSystemComponent.SetVectorParameter` (`self.VFX_Weather_Hail_ForBP`) "Forces" (`KismetMathLibrary.MakeVector` (* (.x (`self.Forces`)) _returnvalue) (* (.y (`self.Forces`)) _returnvalue) (* (.z (`self.Forces`)) (`KismetMathLibrary.RandomFloatInRange` 0.75 1.25)))))

(fn `UserConstructionScript`
  (bind _returnvalue (`PrimitiveComponent.CreateDynamicMaterialInstance` (`self.VFX_Weather_Hail_ForBP`) 0 "/Game/VFX_Weather/VFX_Weather_Materials/Hail_Inst.Hail_Inst"))
  (set `self.HailMat` _returnvalue)
  (`self.HailParameters`))