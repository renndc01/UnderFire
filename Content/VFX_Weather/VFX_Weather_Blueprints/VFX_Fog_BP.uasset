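; Weather VFX actor that renders fog on its Cube2Sphere component with a configurable color and drift direction.
; NewFunction0 creates a dynamic instance of the fog material and writes FogColor and the halved force vector into it as parameters.
; The construction script runs this update unless the actor is a child actor.
; Tick repeats it every frame, calling the dynamic instance creation again each time.
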(event `self.ReceiveBeginPlay`
  (bind _returnvalue (`PrimitiveComponent.CreateDynamicMaterialInstance` (`self.Cube2Sphere`) 0 "/Game/VFX_Weather/VFX_Weather_Materials/Fog_Mat_Inst.Fog_Mat_Inst"))
  (set `self.Fog_Mat` _returnvalue))

(event `self.ReceiveTick`
  (params (DeltaSeconds :type "Float (single-precision)"))
  (`self.NewFunction_0` (`self.Fog Color`) (`self.Forces`)))

(fn `NewFunction_0`
  (params (FogColor :type "LinearColor Structure") (ForceDirection :type "Vector Structure"))
  (bind _returnvalue (`PrimitiveComponent.CreateDynamicMaterialInstance` (`self.Cube2Sphere`) 0 "/Game/VFX_Weather/VFX_Weather_Materials/Fog_Mat_Inst.Fog_Mat_Inst"))
  (set `self.Fog_Mat` _returnvalue)
  (`MaterialInstanceDynamic.SetVectorParameterValue` (`self.Fog_Mat`) "FogColor" FogColor)
  (`MaterialInstanceDynamic.SetVectorParameterValue` (`self.Fog_Mat`) "FogDirection" (`KismetMathLibrary.Conv_VectorToLinearColor` (* ForceDirection 0.5))))

(fn `UserConstructionScript`
  (if (not (`self.IsChildActor`))
    (`self.NewFunction_0` (`self.Fog Color`) (`self.Forces`))))