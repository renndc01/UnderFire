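; Rain VFX actor that drives a particle system's spawn rates, forces and materials from its rain settings.
; Init, run at construction and BeginPlay, creates dynamic materials for drops and splashes, then applies color, emissive, opacity and distortion (drops only).
; The secondary spawn rate is a multiple of SpawnRate, and forces get per-axis random variation.
; Tick reapplies spawn rates, forces and material settings only when SpawnRate changes.
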(event `self.ReceiveBeginPlay`
  (`self.Init`))

(event `self.ReceiveTick`
  (params (DeltaSeconds :type "Float (single-precision)"))
  (bind _returnvalue (`KismetMathLibrary.RandomFloatInRange` 0.5 1.5))
  (if (not (== (`self.LastSpawnRate`) (`self.SpawnRate`)))
    (set `self.LastSpawnRate` (`self.SpawnRate`))
    (`ParticleSystemComponent.SetFloatParameter` (`self.BP_Rain_PS`) "SpawnRate" (`self.SpawnRate`))
    (`ParticleSystemComponent.SetFloatParameter` (`self.BP_Rain_PS`) "SpawnRate2" (* (`self.SpawnRate`) 5.0))
    (`ParticleSystemComponent.SetVectorParameter` (`self.BP_Rain_PS`) "Forces" (`KismetMathLibrary.MakeVector` (* (.x (`self.Forces`)) _returnvalue) (* (.y (`self.Forces`)) _returnvalue) (* (.z (`self.Forces`)) (`KismetMathLibrary.RandomFloatInRange` 0.75 1.25))))
    (`self.RainMaterialFunctionality`)))

(fn `Init`
  (bind _returnvalue (`KismetMathLibrary.RandomFloatInRange` 0.5 1.5))
  (bind _bp_rain_ps (`self.BP_Rain_PS`))
  (bind _spawnrate (`self.SpawnRate`))
  (`ParticleSystemComponent.SetFloatParameter` _bp_rain_ps "SpawnRate" _spawnrate)
  (`ParticleSystemComponent.SetFloatParameter` _bp_rain_ps "SpawnRate2" (* _spawnrate 5.0))
  (bind _returnvalue_2 (`KismetMaterialLibrary.CreateDynamicMaterialInstance` "/Game/VFX_Weather/VFX_Weather_Materials/RainDrop_Inst.RainDrop_Inst"))
  (set `self.RainMat` _returnvalue_2)
  (`PrimitiveComponent.SetMaterial` (`self.BP_Rain_PS`) 0 (`self.RainMat`))
  (`PrimitiveComponent.SetMaterial` (`self.BP_Rain_PS`) 2 (`self.RainMat`))
  (bind _returnvalue_3 (`PrimitiveComponent.CreateDynamicMaterialInstance` (`self.BP_Rain_PS`) 1 "/Game/VFX_Weather/VFX_Weather_Materials/Splash_Inst.Splash_Inst"))
  (set `self.SplashMat` _returnvalue_3)
  (`ParticleSystemComponent.SetVectorParameter` (`self.BP_Rain_PS`) "Forces" (`KismetMathLibrary.MakeVector` (* (.x (`self.Forces`)) _returnvalue) (* (.y (`self.Forces`)) _returnvalue) (* (.z (`self.Forces`)) (`KismetMathLibrary.RandomFloatInRange` 0.75 1.25))))
  (`self.RainMaterialFunctionality`))

(fn `RainMaterialFunctionality`
  (bind _returnvalue (`KismetMathLibrary.RandomFloatInRange` 0.5 1.5))
  (`ParticleSystemComponent.SetVectorParameter` (`self.BP_Rain_PS`) "Forces" (`KismetMathLibrary.MakeVector` (* (.x (`self.Forces`)) _returnvalue) (* (.y (`self.Forces`)) _returnvalue) (* (.z (`self.Forces`)) (`KismetMathLibrary.RandomFloatInRange` 0.75 1.25))))
  (`MaterialInstanceDynamic.SetVectorParameterValue` (`self.RainMat`) "RainColor" (`self.RainColor`))
  (`MaterialInstanceDynamic.SetScalarParameterValue` (`self.RainMat`) "Emissive" (`self.Emissive`))
  (`MaterialInstanceDynamic.SetScalarParameterValue` (`self.RainMat`) "RainOpacity" (`self.Opacity`))
  (`MaterialInstanceDynamic.SetScalarParameterValue` (`self.RainMat`) "RainDistortion" (`self.Distortion`))
  (`MaterialInstanceDynamic.SetVectorParameterValue` (`self.SplashMat`) "LiquidColor" (`self.RainColor`))
  (`MaterialInstanceDynamic.SetScalarParameterValue` (`self.SplashMat`) "Emissive" (`self.Emissive`))
  (`MaterialInstanceDynamic.SetScalarParameterValue` (`self.SplashMat`) "Opacity" (* (`self.Opacity`) 0.2)))

(fn `UserConstructionScript`
  (`self.Init`))