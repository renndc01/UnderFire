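; Weather effect actor that drives a snow particle component with configurable spawn rate and force settings.
; The construction script pushes both values to the particle parameters, so edits show in the editor.
; Every tick it reapplies them, scaling the force vector by a new random factor around its base value to give a gusty, uneven drift.
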(event `self.ReceiveTick`
  (params (DeltaSeconds :type "Float (single-precision)"))
  (`ParticleSystemComponent.SetFloatParameter` (`self.VFX_Weather_Snow_ForBP`) "SpawnRate" (`self.SpawnRate`))
  (`ParticleSystemComponent.SetVectorParameter` (`self.VFX_Weather_Snow_ForBP`) "Forces" (* (`self.Forces`) (`KismetMathLibrary.RandomFloatInRange` 0.5 1.5))))

(fn `UserConstructionScript`
  (`ParticleSystemComponent.SetFloatParameter` (`self.VFX_Weather_Snow_ForBP`) "SpawnRate" (`self.SpawnRate`))
  (`ParticleSystemComponent.SetVectorParameter` (`self.VFX_Weather_Snow_ForBP`) "Forces" (`self.Forces`)))