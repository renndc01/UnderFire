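; Twin iron street lamp pole with configurable paint color, rust spread, light and light shaft.
; The construction script creates dynamic material instances for the pole's LOD material slots and applies paint and rust.
; When lit, it sets spotlight brightness, makes bulb and glass emissive, and toggles spotlight and optional shaft visibility.
; BeginPlay always destroys the SpotLight, leaving it out of runtime, and removes the shaft mesh if disabled.
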(event EventBeginPlay
  ;[1 1 1] Destroy the SpotLight
  (Components|DestroyComponent (Variables|Default|GetSpotLight))
  ;[1 1 1] Switch between light OFF and ON
  (if (not (Variables|Default|GetLightshaft%20ON/OFF))
    ;[1 1 1] If the light is switched off the Lightshaft becomes unnecessary
    (Components|DestroyComponent (Variables|Default|GetSM_Lightshaft))))

(fn ConstructionScript
  ;[1 1 1] Create DMI for all LOD
  (bind _returnvalue (Rendering|Material|CreateDynamicMaterialInstance (Variables|Default|GetSM_ipTwinG) 0 "/Game/streetLights/Materials/M_ironpoleTWIN_Inst.M_ironpoleTWIN_Inst" :!class /Script/Engine.PrimitiveComponent))
  (LocalVariables|SetMI_ironpoleTWIN_EI_0 _returnvalue)
  (bind _returnvalue_2 (Rendering|Material|CreateDynamicMaterialInstance (Variables|Default|GetSM_ipTwinG) 2 "/Game/streetLights/Materials/M_ironpoleTWIN_Inst.M_ironpoleTWIN_Inst" :!class /Script/Engine.PrimitiveComponent))
  (LocalVariables|SetMI_ironpoleTWIN_EI_2 _returnvalue_2)
  (bind _returnvalue_3 (Rendering|Material|CreateDynamicMaterialInstance (Variables|Default|GetSM_ipTwinG) 4 "/Game/streetLights/Materials/M_ironpoleTWIN_Inst.M_ironpoleTWIN_Inst" :!class /Script/Engine.PrimitiveComponent))
  (LocalVariables|SetMI_ironpoleTWIN_EI_4 _returnvalue_3)
  ;[1 1 1] Set the Paint Color parameter for all LOD
  (Rendering|Material|SetVectorParameterValue (LocalVariables|GetMI_ironpoleTWIN_EI_0) "Paint_color" (Variables|Default|GetPaint%20Color) :!class /Script/Engine.MaterialInstanceDynamic)
  (Rendering|Material|SetVectorParameterValue (LocalVariables|GetMI_ironpoleTWIN_EI_2) "Paint_color" (Variables|Default|GetPaint%20Color) :!class /Script/Engine.MaterialInstanceDynamic)
  (Rendering|Material|SetVectorParameterValue (LocalVariables|GetMI_ironpoleTWIN_EI_4) "Paint_color" (Variables|Default|GetPaint%20Color) :!class /Script/Engine.MaterialInstanceDynamic)
  ;[1 1 1] Set the Rust_spread parameter for all LOD
  (Rendering|Material|SetScalarParameterValue (LocalVariables|GetMI_ironpoleTWIN_EI_0) "Rust_spread" (Variables|Default|GetRust%20Spread) :!class /Script/Engine.MaterialInstanceDynamic)
  (Rendering|Material|SetScalarParameterValue (LocalVariables|GetMI_ironpoleTWIN_EI_2) "Rust_spread" (Variables|Default|GetRust%20Spread) :!class /Script/Engine.MaterialInstanceDynamic)
  (Rendering|Material|SetScalarParameterValue (LocalVariables|GetMI_ironpoleTWIN_EI_4) "Rust_spread" (Variables|Default|GetRust%20Spread) :!class /Script/Engine.MaterialInstanceDynamic)
  ;[1 1 1] Control the lighting
  (if (Variables|Default|GetLight%20ON/OFF)
    ;[1 1 1] Set the Spotlight light intensity
    (Rendering|Components|Light|SetIntensity (Variables|Default|GetSpotLight) (Variables|Default|GetBrightness))
    ;[1 1 1] Set the Spotlight Visibility to true
    (Rendering|ToggleVisibility (Variables|Default|GetSpotLight) false)
    ;[1 1 1] Set the Bulb emission for all LOD
    (Rendering|Material|SetScalarParameterValue (LocalVariables|GetMI_ironpoleTWIN_EI_0) "Light_Strength" 5e+01 :!class /Script/Engine.MaterialInstanceDynamic)
    (Rendering|Material|SetScalarParameterValue (LocalVariables|GetMI_ironpoleTWIN_EI_2) "Light_Strength" 5e+01 :!class /Script/Engine.MaterialInstanceDynamic)
    (Rendering|Material|SetScalarParameterValue (LocalVariables|GetMI_ironpoleTWIN_EI_4) "Light_Strength" 5e+01 :!class /Script/Engine.MaterialInstanceDynamic)
    ;[1 1 1] Create Glass DMI and set to emit for all LOD
    (bind _returnvalue_4 (Rendering|Material|CreateDynamicMaterialInstance (Variables|Default|GetSM_ipTwinG) 1 "/Game/streetLights/Materials/M_glass_Inst.M_glass_Inst" :!class /Script/Engine.PrimitiveComponent))
    (Rendering|Material|SetScalarParameterValue _returnvalue_4 "Light_strength" 2.0 :!class /Script/Engine.MaterialInstanceDynamic)
    (bind _returnvalue_5 (Rendering|Material|CreateDynamicMaterialInstance (Variables|Default|GetSM_ipTwinG) 3 "/Game/streetLights/Materials/M_glass_Inst.M_glass_Inst" :!class /Script/Engine.PrimitiveComponent))
    (Rendering|Material|SetScalarParameterValue _returnvalue_5 "Light_strength" 2.0 :!class /Script/Engine.MaterialInstanceDynamic)
    (bind _returnvalue_6 (Rendering|Material|CreateDynamicMaterialInstance (Variables|Default|GetSM_ipTwinG) 5 "/Game/streetLights/Materials/M_glass_Inst.M_glass_Inst" :!class /Script/Engine.PrimitiveComponent))
    (Rendering|Material|SetScalarParameterValue _returnvalue_6 "Light_strength" 2.0 :!class /Script/Engine.MaterialInstanceDynamic)
    ;[1 1 1] Controll the lightshaft
    (if (Variables|Default|GetLightshaft%20ON/OFF)
      ;[1 1 1] Set the Lightshaft Visibility to true
      (Rendering|ToggleVisibility (Variables|Default|GetSM_Lightshaft) false))))