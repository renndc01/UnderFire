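; Configurable twin wooden-pole street light prop with a spotlight, emissive bulb and optional lightshaft mesh.
; The construction script creates dynamic material instances on three material slots, one per LOD, to apply paint color, rust spread and wood age.
; When switched on, it also sets spotlight intensity and bulb emission, and toggles spotlight and optional lightshaft visibility.
; BeginPlay always destroys the SpotLight component, and removes the lightshaft if the light is off.
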(event `self.ReceiveBeginPlay`
  ;[1 1 1] Destroy the SpotLight
  (`ActorComponent.K2_DestroyComponent` (`self.SpotLight`))
  ;[1 1 1] Switch between light OFF and ON
  (if (not (`self.Light ON/OFF`))
    ;[1 1 1] If the light is switched off the Lightshaft becomes unnecessary
    (`ActorComponent.K2_DestroyComponent` (`self.SM_Lightshaft`))))

(fn `UserConstructionScript`
  (locals (MI_woodenpoleTWIN_EI_0 :type "MaterialInstanceDynamic Object Reference") (MI_woodenpoleTWIN_EI_1 :type "MaterialInstanceDynamic Object Reference") (MI_woodenpoleTWIN_EI_2 :type "MaterialInstanceDynamic Object Reference"))
  ;[1 1 1] Create DMI for all LOD
  (bind _returnvalue (`PrimitiveComponent.CreateDynamicMaterialInstance` (`self.SM_wpTWIN`) 0 "/Game/streetLights/Materials/M_woodenpoleTWIN_Inst.M_woodenpoleTWIN_Inst"))
  (set `local.MI_woodenpoleTWIN_EI_0` _returnvalue)
  (bind _returnvalue_2 (`PrimitiveComponent.CreateDynamicMaterialInstance` (`self.SM_wpTWIN`) 1 "/Game/streetLights/Materials/M_woodenpoleTWIN_Inst.M_woodenpoleTWIN_Inst"))
  (set `local.MI_woodenpoleTWIN_EI_1` _returnvalue_2)
  (bind _returnvalue_3 (`PrimitiveComponent.CreateDynamicMaterialInstance` (`self.SM_wpTWIN`) 2 "/Game/streetLights/Materials/M_woodenpoleTWIN_Inst.M_woodenpoleTWIN_Inst"))
  (set `local.MI_woodenpoleTWIN_EI_2` _returnvalue_3)
  ;[1 1 1] Set the Paint Color parameter for all LOD
  (`MaterialInstanceDynamic.SetVectorParameterValue` (`local.MI_woodenpoleTWIN_EI_0`) "Paint_color" (`self.Paint color`))
  (`MaterialInstanceDynamic.SetVectorParameterValue` (`local.MI_woodenpoleTWIN_EI_1`) "Paint_color" (`self.Paint color`))
  (`MaterialInstanceDynamic.SetVectorParameterValue` (`local.MI_woodenpoleTWIN_EI_2`) "Paint_color" (`self.Paint color`))
  ;[1 1 1] Set the Rust_spread parameter for all LOD
  (`MaterialInstanceDynamic.SetScalarParameterValue` (`local.MI_woodenpoleTWIN_EI_0`) "Rust_spread" (`self.Rust Spread`))
  (`MaterialInstanceDynamic.SetScalarParameterValue` (`local.MI_woodenpoleTWIN_EI_1`) "Rust_spread" (`self.Rust Spread`))
  (`MaterialInstanceDynamic.SetScalarParameterValue` (`local.MI_woodenpoleTWIN_EI_2`) "Rust_spread" (`self.Rust Spread`))
  ;[1 1 1] Set the Wood_age parameter for all LOD
  (`MaterialInstanceDynamic.SetScalarParameterValue` (`local.MI_woodenpoleTWIN_EI_0`) "Wood_age" (`self.Wood age`))
  (`MaterialInstanceDynamic.SetScalarParameterValue` (`local.MI_woodenpoleTWIN_EI_1`) "Wood_age" (`self.Wood age`))
  (`MaterialInstanceDynamic.SetScalarParameterValue` (`local.MI_woodenpoleTWIN_EI_2`) "Wood_age" (`self.Wood age`))
  ;[1 1 1] Controll the lighting
  (if (`self.Light ON/OFF`)
    ;[1 1 1] Set the Spotlight light intensity
    (`LightComponent.SetIntensity` (`self.SpotLight`) (`self.Brightness`))
    ;[1 1 1] Set the Spotlight Visibility to true
    (`SceneComponent.ToggleVisibility` (`self.SpotLight`) false)
    ;[1 1 1] Set the Bulb emission for all LOD
    (`MaterialInstanceDynamic.SetScalarParameterValue` (`local.MI_woodenpoleTWIN_EI_0`) "Light_Strength" 50.0)
    (`MaterialInstanceDynamic.SetScalarParameterValue` (`local.MI_woodenpoleTWIN_EI_1`) "Light_Strength" 50.0)
    (`MaterialInstanceDynamic.SetScalarParameterValue` (`local.MI_woodenpoleTWIN_EI_2`) "Light_Strength" 50.0)
    ;[1 1 1] Controll the lightshaft
    (if (`self.Lightshaft ON/OFF`)
      ;[1 1 1] Set the Lightshaft Visibility to true
      (`SceneComponent.ToggleVisibility` (`self.SM_Lightshaft`) false))))