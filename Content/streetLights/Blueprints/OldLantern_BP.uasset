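; Old lantern street light prop with configurable paint color, rust, dirt and an on/off light.
; The construction script creates dynamic body materials on three slots, one per LOD, and applies the appearance settings.
; When the light is on, it sets point light brightness, toggles its visibility and makes bulb and glass materials emissive.
; BeginPlay destroys the point light, so only the emissive materials remain dynamically lit-looking during play.
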(event EventBeginPlay
  ;[1 1 1] Destroy the pointlight
  (Components|DestroyComponent (Variables|Default|GetPointLight)))

(fn ConstructionScript
  ;[1 1 1] Create DMI for all LOD
  (bind _returnvalue (Rendering|Material|CreateDynamicMaterialInstance (Variables|Default|GetStaticMesh) 0 "/Game/streetLights/Materials/M_OldLantern_Inst.M_OldLantern_Inst" :!class /Script/Engine.PrimitiveComponent))
  (LocalVariables|SetMI_OldLantern_EI_0 _returnvalue)
  (bind _returnvalue_2 (Rendering|Material|CreateDynamicMaterialInstance (Variables|Default|GetStaticMesh) 2 "/Game/streetLights/Materials/M_OldLantern_Inst.M_OldLantern_Inst" :!class /Script/Engine.PrimitiveComponent))
  (LocalVariables|SetMI_OldLantern_EI_2 _returnvalue_2)
  (bind _returnvalue_3 (Rendering|Material|CreateDynamicMaterialInstance (Variables|Default|GetStaticMesh) 4 "/Game/streetLights/Materials/M_OldLantern_Inst.M_OldLantern_Inst" :!class /Script/Engine.PrimitiveComponent))
  (LocalVariables|SetMI_OldLantern_EI_4 _returnvalue_3)
  ;[1 1 1] Set the Paint Color parameter for all LOD
  (Rendering|Material|SetVectorParameterValue (LocalVariables|GetMI_OldLantern_EI_0) "Paint_color" (Variables|Default|GetPaint%20Color) :!class /Script/Engine.MaterialInstanceDynamic)
  (Rendering|Material|SetVectorParameterValue (LocalVariables|GetMI_OldLantern_EI_2) "Paint_color" (Variables|Default|GetPaint%20Color) :!class /Script/Engine.MaterialInstanceDynamic)
  (Rendering|Material|SetVectorParameterValue (LocalVariables|GetMI_OldLantern_EI_4) "Paint_color" (Variables|Default|GetPaint%20Color) :!class /Script/Engine.MaterialInstanceDynamic)
  ;[1 1 1] Set the Rust_spread parameter for all LOD
  (Rendering|Material|SetScalarParameterValue (LocalVariables|GetMI_OldLantern_EI_0) "Rust_spread" (Variables|Default|GetRust%20Spread) :!class /Script/Engine.MaterialInstanceDynamic)
  (Rendering|Material|SetScalarParameterValue (LocalVariables|GetMI_OldLantern_EI_2) "Rust_spread" (Variables|Default|GetRust%20Spread) :!class /Script/Engine.MaterialInstanceDynamic)
  (Rendering|Material|SetScalarParameterValue (LocalVariables|GetMI_OldLantern_EI_4) "Rust_spread" (Variables|Default|GetRust%20Spread) :!class /Script/Engine.MaterialInstanceDynamic)
  ;[1 1 1] Set the Dirt_spread parameter for all LOD
  (Rendering|Material|SetScalarParameterValue (LocalVariables|GetMI_OldLantern_EI_0) "Dirt_spread" (Variables|Default|GetDirt%20Spread) :!class /Script/Engine.MaterialInstanceDynamic)
  (Rendering|Material|SetScalarParameterValue (LocalVariables|GetMI_OldLantern_EI_2) "Dirt_spread" (Variables|Default|GetDirt%20Spread) :!class /Script/Engine.MaterialInstanceDynamic)
  (Rendering|Material|SetScalarParameterValue (LocalVariables|GetMI_OldLantern_EI_4) "Dirt_spread" (Variables|Default|GetDirt%20Spread) :!class /Script/Engine.MaterialInstanceDynamic)
  ;[1 1 1] Controll the lighting
  (if (Variables|Default|GetLight%20ON/OFF)
    ;[1 1 1] Set the intensity of the pointlight
    (Rendering|Components|Light|SetIntensity (Variables|Default|GetPointLight) (Variables|Default|GetBrightness))
    ;[1 1 1] Set the Pointlight Visibility to true
    (Rendering|ToggleVisibility (Variables|Default|GetPointLight) false)
    ;[1 1 1] Set the Bulb emission for all LOD
    (Rendering|Material|SetScalarParameterValue (LocalVariables|GetMI_OldLantern_EI_0) "Light_Strength" 0.8 :!class /Script/Engine.MaterialInstanceDynamic)
    (Rendering|Material|SetScalarParameterValue (LocalVariables|GetMI_OldLantern_EI_2) "Light_Strength" 0.8 :!class /Script/Engine.MaterialInstanceDynamic)
    (Rendering|Material|SetScalarParameterValue (LocalVariables|GetMI_OldLantern_EI_4) "Light_Strength" 0.8 :!class /Script/Engine.MaterialInstanceDynamic)
    ;[1 1 1] Create Glass DMI and set to emit for all LOD
    (bind _returnvalue_4 (Rendering|Material|CreateDynamicMaterialInstance (Variables|Default|GetStaticMesh) 1 "/Game/streetLights/Materials/M_OldLanternGlass_Inst.M_OldLanternGlass_Inst" :!class /Script/Engine.PrimitiveComponent))
    (Rendering|Material|SetScalarParameterValue _returnvalue_4 "Light_Strength" 0.9 :!class /Script/Engine.MaterialInstanceDynamic)
    (bind _returnvalue_5 (Rendering|Material|CreateDynamicMaterialInstance (Variables|Default|GetStaticMesh) 3 "/Game/streetLights/Materials/M_OldLanternGlass_Inst.M_OldLanternGlass_Inst" :!class /Script/Engine.PrimitiveComponent))
    (Rendering|Material|SetScalarParameterValue _returnvalue_5 "Light_strength" 0.9 :!class /Script/Engine.MaterialInstanceDynamic)
    (bind _returnvalue_6 (Rendering|Material|CreateDynamicMaterialInstance (Variables|Default|GetStaticMesh) 5 "/Game/streetLights/Materials/M_OldLanternGlass_Inst.M_OldLanternGlass_Inst" :!class /Script/Engine.PrimitiveComponent))
    (Rendering|Material|SetScalarParameterValue _returnvalue_6 "Light_strength" 0.9 :!class /Script/Engine.MaterialInstanceDynamic)))