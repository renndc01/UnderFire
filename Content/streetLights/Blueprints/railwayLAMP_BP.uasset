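; Railway lamp Blueprint, a street light prop with adjustable rust, an on/off switch and an optional light shaft mesh.
; The construction script creates dynamic materials for two material slots, sets rust spread, and when lit sets spotlight brightness, bulb emission and visibility toggles.
; BeginPlay always destroys the SpotLight, leaving it only for editor time, and also removes the light shaft if the lamp is off.
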(event EventBeginPlay
  ;[1 1 1] Destroy the SpotLight
  (Components|DestroyComponent (Variables|Default|GetSpotLight))
  ;[1 1 1] Switch between light OFF and ON
  (if (not (Variables|Default|GetLight%20ON/OFF))
    ;[1 1 1] If the light is switched off the Lightshaft becomes unnecessary
    (Components|DestroyComponent (Variables|Default|GetSM_Lightshaft))))

(fn ConstructionScript
  ;[1 1 1] Create DMI for all LOD
  (bind _returnvalue (Rendering|Material|CreateDynamicMaterialInstance (Variables|Default|GetSM_rwLAMP) 0 "/Game/streetLights/Materials/M_railwayLAMP_Inst.M_railwayLAMP_Inst" :!class /Script/Engine.PrimitiveComponent))
  (LocalVariables|SetMI_railwayLAMP_EI_0 _returnvalue)
  (bind _returnvalue_2 (Rendering|Material|CreateDynamicMaterialInstance (Variables|Default|GetSM_rwLAMP) 1 "/Game/streetLights/Materials/M_railwayLAMP_Inst.M_railwayLAMP_Inst" :!class /Script/Engine.PrimitiveComponent))
  (LocalVariables|SetMI_railwayLAMP_EI_1 _returnvalue_2)
  ;[1 1 1] Set the Rust_spread parameter for all LOD
  (Rendering|Material|SetScalarParameterValue (LocalVariables|GetMI_railwayLAMP_EI_0) "Rust_spread" (Variables|Default|GetRust%20Spread) :!class /Script/Engine.MaterialInstanceDynamic)
  (Rendering|Material|SetScalarParameterValue (LocalVariables|GetMI_railwayLAMP_EI_1) "Rust_spread" (Variables|Default|GetRust%20Spread) :!class /Script/Engine.MaterialInstanceDynamic)
  ;[1 1 1] Control the lighting
  (if (Variables|Default|GetLight%20ON/OFF)
    ;[1 1 1] Set the Spotlight light intensity
    (Rendering|Components|Light|SetIntensity (Variables|Default|GetSpotLight) (Variables|Default|GetBrightness))
    ;[1 1 1] Set the Spotlight Visibility to true
    (Rendering|ToggleVisibility (Variables|Default|GetSpotLight) false)
    ;[1 1 1] Set the Bulb emission for all LOD
    (Rendering|Material|SetScalarParameterValue (LocalVariables|GetMI_railwayLAMP_EI_0) "Light_Strength" 5e+01 :!class /Script/Engine.MaterialInstanceDynamic)
    (Rendering|Material|SetScalarParameterValue (LocalVariables|GetMI_railwayLAMP_EI_1) "Light_Strength" 5e+01 :!class /Script/Engine.MaterialInstanceDynamic)
    ;[1 1 1] Controll the lightshaft
    (if (Variables|Default|GetLightshaft%20ON/OFF)
      ;[1 1 1] Set the Lightshaft Visibility to true
      (Rendering|ToggleVisibility (Variables|Default|GetSM_Lightshaft) false))))