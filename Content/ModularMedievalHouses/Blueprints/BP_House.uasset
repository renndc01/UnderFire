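; Modular medieval house actor that assembles itself in the construction script from exposed options.
; It places optional wings and extensions, then adds balconies, staircases and doors at named window sockets, and chimneys at listed transforms.
; Component tags drive dynamic material instances that apply a shared Age parameter, plus a roof texture choice.
; It also sets meshes to WorldStatic and can label sockets with text renders for placement.
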(fn `UserConstructionScript`
  (bind _doorlocation (`self.DoorLocation`))
  (bind _chimney (`self.Chimney`))
  (bind _age (`self.Age`))
  (bind _age_2 (`self.Age`))
  (bind _age_3 (`self.Age`))
  (bind _staticmesh (`self.StaticMesh`))
  (bind _wingdoorlocation (`self.WingDoorLocation`))
  (bind _extention1_0 (`self.Extention1.0`))
  (bind _extention1_0_2 (`self.Extention1.0`))
  (bind _extention1_1 (`self.Extention1.1`))
  (bind _extention2_1 (`self.Extention2.1`))
  (bind _extention2_0 (`self.Extention2.0`))
  (bind _extention2_0_2 (`self.Extention2.0`))
  (bind _main_building_balcony (`self.Main Building Balcony`))
  (bind _age_4 (`self.Age`))
  (bind _wingbalcony (`self.WingBalcony`))
  (bind _returnvalue (`KismetArrayLibrary.Array_Length` _main_building_balcony))
  (bind _returnvalue_2 (`KismetArrayLibrary.Array_Length` _doorlocation))
  (bind _returnvalue_3 (`KismetArrayLibrary.Array_Length` _chimney))
  (`|ExecutionSequence`
    (:`then_0`
      ;[1 1 1] Extentions
      (if (`self.EnableExtention1`)
        (if (<= (`self.Extention1 Amount`) 1)
          (`StaticMeshComponent.SetStaticMesh` _extention1_0 (select `int` (`self.Extention1 Type`) :`0` "/Game/ModularMedievalHouses/Meshes/SM_HousePart1.SM_HousePart1" :`1` "/Game/ModularMedievalHouses/Meshes/SM_HousePart2.SM_HousePart2" :!type "StaticMesh Object Reference"))
          (`SceneComponent.K2_SetRelativeLocation` _extention1_0 (-4.0 406.0 0.0) false false)
          (else
            (`StaticMeshComponent.SetStaticMesh` _extention1_0_2 (select `int` (`self.Extention1 Type`) :`0` "/Game/ModularMedievalHouses/Meshes/SM_HousePart1.SM_HousePart1" :`1` "/Game/ModularMedievalHouses/Meshes/SM_HousePart2.SM_HousePart2" :!type "StaticMesh Object Reference"))
            (`SceneComponent.K2_SetRelativeLocation` _extention1_0_2 (-247.0 406.0 0.0) false false)
            (`StaticMeshComponent.SetStaticMesh` _extention1_1 (select `int` (`self.Extention1.1 Type`) :`0` "/Game/ModularMedievalHouses/Meshes/SM_HousePart1.SM_HousePart1" :`1` "/Game/ModularMedievalHouses/Meshes/SM_HousePart2.SM_HousePart2" :!type "StaticMesh Object Reference"))
            (`SceneComponent.K2_SetRelativeLocation` _extention1_1 (247.0 406.0 0.0) false false)))))
    (:`then_1`
      (if (`self.EnableExtention2`)
        (if (<= (`self.Extention2 Amount`) 1)
          (`StaticMeshComponent.SetStaticMesh` _extention2_0_2 (select `int` (`self.Extention2 Type`) :`0` "/Game/ModularMedievalHouses/Meshes/SM_HousePart1.SM_HousePart1" :`1` "/Game/ModularMedievalHouses/Meshes/SM_HousePart2.SM_HousePart2" :!type "StaticMesh Object Reference"))
          (`SceneComponent.K2_SetRelativeLocation` _extention2_0_2 (-4.0 -406.0 0.0) false false)
          (else
            (`StaticMeshComponent.SetStaticMesh` _extention2_0 (select `int` (`self.Extention2 Type`) :`0` "/Game/ModularMedievalHouses/Meshes/SM_HousePart1.SM_HousePart1" :`1` "/Game/ModularMedievalHouses/Meshes/SM_HousePart2.SM_HousePart2" :!type "StaticMesh Object Reference"))
            (`SceneComponent.K2_SetRelativeLocation` _extention2_0 (-247.0 -406.0 0.0) false false)
            (`StaticMeshComponent.SetStaticMesh` _extention2_1 (select `int` (`self.Extention2.1 Type`) :`0` "/Game/ModularMedievalHouses/Meshes/SM_HousePart1.SM_HousePart1" :`1` "/Game/ModularMedievalHouses/Meshes/SM_HousePart2.SM_HousePart2" :!type "StaticMesh Object Reference"))
            (`SceneComponent.K2_SetRelativeLocation` _extention2_1 (247.0 -406.0 0.0) false false)))))
    (:`then_2`
      ;[1 1 1] Wings
      (`StaticMeshComponent.SetStaticMesh` (`self.LeftWing`) (select `bool` (`self.EnableLeftWing`) :`true` (select `int` (`self.LeftWingType`) :`0` "/Game/ModularMedievalHouses/Meshes/SM_HousePart1.SM_HousePart1" :`1` "/Game/ModularMedievalHouses/Meshes/SM_HousePart2.SM_HousePart2" :!type "StaticMesh Object Reference")))
      (`StaticMeshComponent.SetStaticMesh` (`self.RightWing`) (select `bool` (`self.EnableRightWing`) :`true` (select `int` (`self.RightWingType`) :`0` "/Game/ModularMedievalHouses/Meshes/SM_HousePart1.SM_HousePart1" :`1` "/Game/ModularMedievalHouses/Meshes/SM_HousePart2.SM_HousePart2" :!type "StaticMesh Object Reference")))
      (`SceneComponent.K2_SetRelativeTransform` (`self.LeftWing`) (`KismetMathLibrary.MakeTransform` (-596.0 0.0 0.0) (struct :`Yaw` 90.0)) false false)
      (`SceneComponent.K2_SetRelativeTransform` (`self.RightWing`) (`KismetMathLibrary.MakeTransform` (596.0 0.0 0.0) (struct :`Yaw` -90.0)) false false))
    (:`then_4`
      ;[1 1 1] Balcony
      (`|ExecutionSequence`
        (:`then_0`
          (if (> _returnvalue 0)
            (for _index (range _returnvalue)
              (bind (_balconylocation _balconytype) (break `/Game/ModularMedievalHouses/Blueprints/EnumsAndStructs/BalconyStructure` (`KismetArrayLibrary.Array_Get` _main_building_balcony _index)))
              (bind _returnvalue_4 (`AddComponent|StaticMeshComponent_13` :`RelativeTransform` (`KismetMathLibrary.MakeTransform` (`KismetMathLibrary.MakeVector` (select `/Game/ModularMedievalHouses/Blueprints/EnumsAndStructs/BalconyType` _balconytype :`NewEnumerator0` (.x (.location (`SceneComponent.GetSocketTransform` (`self.StaticMesh`) (select `/Game/ModularMedievalHouses/Blueprints/EnumsAndStructs/BalconyLocation` _balconylocation :`NewEnumerator0` "Window5" :`NewEnumerator1` "Window6" :`NewEnumerator2` "Window7" :`NewEnumerator3` "Window8" :`NewEnumerator4` "Window9" :`NewEnumerator5` "Window10" :!type "Name") "RTS_Actor")))) (.y (.location (`SceneComponent.GetSocketTransform` (`self.StaticMesh`) (select `/Game/ModularMedievalHouses/Blueprints/EnumsAndStructs/BalconyLocation` _balconylocation :`NewEnumerator0` "Window5" :`NewEnumerator1` "Window6" :`NewEnumerator2` "Window7" :`NewEnumerator3` "Window8" :`NewEnumerator4` "Window9" :`NewEnumerator5` "Window10" :!type "Name") "RTS_Actor"))) (.z (.location (`SceneComponent.GetSocketTransform` (`self.StaticMesh`) (select `/Game/ModularMedievalHouses/Blueprints/EnumsAndStructs/BalconyLocation` _balconylocation :`NewEnumerator0` "Window5" :`NewEnumerator1` "Window6" :`NewEnumerator2` "Window7" :`NewEnumerator3` "Window8" :`NewEnumerator4` "Window9" :`NewEnumerator5` "Window10" :!type "Name") "RTS_Actor")))) (.rotation (`SceneComponent.GetSocketTransform` (`self.StaticMesh`) (select `/Game/ModularMedievalHouses/Blueprints/EnumsAndStructs/BalconyLocation` _balconylocation :`NewEnumerator0` "Window5" :`NewEnumerator1` "Window6" :`NewEnumerator2` "Window7" :`NewEnumerator3` "Window8" :`NewEnumerator4` "Window9" :`NewEnumerator5` "Window10" :!type "Name") "RTS_Actor")) (.scale (`SceneComponent.GetSocketTransform` (`self.StaticMesh`) (select `/Game/ModularMedievalHouses/Blueprints/EnumsAndStructs/BalconyLocation` _balconylocation :`NewEnumerator0` "Window5" :`NewEnumerator1` "Window6" :`NewEnumerator2` "Window7" :`NewEnumerator3` "Window8" :`NewEnumerator4` "Window9" :`NewEnumerator5` "Window10" :!type "Name") "RTS_Actor")))))
              (`KismetArrayLibrary.Array_Add` (`ActorComponent.ComponentTags` _returnvalue_4) "Balcony")
              (`StaticMeshComponent.SetStaticMesh` _returnvalue_4 (select `/Game/ModularMedievalHouses/Blueprints/EnumsAndStructs/BalconyType` _balconytype :`NewEnumerator0` "/Game/ModularMedievalHouses/Meshes/SM_SmallBalcony.SM_SmallBalcony" :`NewEnumerator1` "/Game/ModularMedievalHouses/Meshes/SM_LargeBalcony.SM_LargeBalcony" :`NewEnumerator2` "/Game/ModularMedievalHouses/Meshes/SM_Staircase1.SM_Staircase1" :`NewEnumerator3` "/Game/ModularMedievalHouses/Meshes/SM_Staircase2.SM_Staircase2" :`NewEnumerator4` "/Game/ModularMedievalHouses/Meshes/SM_Staircase3.SM_Staircase3" :!type "StaticMesh Object Reference")))))
        (:`then_1`
          (if (> (`KismetArrayLibrary.Array_Length` _wingbalcony) 0)
            (for _array_element _wingbalcony
              (bind (_location _extention) (break `/Game/ModularMedievalHouses/Blueprints/EnumsAndStructs/WingBalconyStructure` _array_element))
              (bind _returnvalue_5 (select `/Game/ModularMedievalHouses/Blueprints/EnumsAndStructs/ExtentionEnum` _extention :`NewEnumerator0` (`self.LeftWing`) :`NewEnumerator1` (`self.RightWing`) :`NewEnumerator2` (`self.Extention1.0`) :`NewEnumerator3` (`self.Extention1.1`) :`NewEnumerator4` (`self.Extention2.0`) :`NewEnumerator5` (`self.Extention2.1`) :!type "SceneComponent Object Reference"))
              (bind _returnvalue_6 (`AddComponent|Static Mesh Component_380` :`RelativeTransform` (`SceneComponent.GetSocketTransform` _returnvalue_5 (select `/Game/ModularMedievalHouses/Blueprints/EnumsAndStructs/WingEnum` _location :`NewEnumerator0` "Window1" :`NewEnumerator1` "Window2" :`NewEnumerator2` "Window3" :`NewEnumerator3` "Window4" :`NewEnumerator4` "Window5" :`NewEnumerator5` "Window6" :!type "Name") "RTS_Actor")))
              (if (== (`SceneComponent.GetRelativeTransform` _returnvalue_6) (`SceneComponent.GetRelativeTransform` _returnvalue_5))
                (`ActorComponent.K2_DestroyComponent` _returnvalue_6)
                (else
                  (`KismetArrayLibrary.Array_Add` (`ActorComponent.ComponentTags` _returnvalue_6) "Balcony")
                  (`StaticMeshComponent.SetStaticMesh` _returnvalue_6 "/Game/ModularMedievalHouses/Meshes/SM_SmallBalcony.SM_SmallBalcony"))))))))
    (:`then_5`
      ;[1 1 1] Doors
      (`|ExecutionSequence`
        (:`then_0`
          (if (> _returnvalue_2 0)
            (for _index_2 (range _returnvalue_2)
              (bind (_doortype _doorlocation_2) (break `/Game/ModularMedievalHouses/Blueprints/EnumsAndStructs/DoorStructure` (`KismetArrayLibrary.Array_Get` _doorlocation _index_2)))
              (bind _returnvalue_7 (`AddComponent|Static Mesh Component_22` :`RelativeTransform` (`SceneComponent.GetSocketTransform` (`self.StaticMesh`) (select `/Game/ModularMedievalHouses/Blueprints/EnumsAndStructs/DoorEnum` _doorlocation_2 :`NewEnumerator0` "Window1" :`NewEnumerator1` "Window2" :`NewEnumerator2` "Window3" :`NewEnumerator3` "Window4" :`NewEnumerator4` "Window5" :`NewEnumerator5` "Window6" :`NewEnumerator6` "Window7" :`NewEnumerator7` "Window8" :`NewEnumerator8` "Window9" :`NewEnumerator9` "Window10" :`NewEnumerator10` "Window11" :`NewEnumerator11` "Window12" :!type "Name") "RTS_Actor")))
              (bind _returnvalue_8 (select `/Game/ModularMedievalHouses/Blueprints/EnumsAndStructs/DoorTypeEnum` _doortype :`NewEnumerator0` "/Game/ModularMedievalHouses/Meshes/SM_StoneFrameDoor.SM_StoneFrameDoor" :`NewEnumerator1` "/Game/ModularMedievalHouses/Meshes/SM_WoodframeDoor.SM_WoodframeDoor" :!type "StaticMesh Object Reference"))
              (`KismetArrayLibrary.Array_Add` (`ActorComponent.ComponentTags` _returnvalue_7) (`KismetStringLibrary.Conv_StringToName` (`KismetStringLibrary.BuildString_Object` "" "" _returnvalue_8)))
              (`StaticMeshComponent.SetStaticMesh` _returnvalue_7 _returnvalue_8))))
        (:`then_1`
          (if (> (`KismetArrayLibrary.Array_Length` _wingdoorlocation) 0)
            (for _array_element_2 _wingdoorlocation
              (bind (_door _location_2 _extention_2) (break `/Game/ModularMedievalHouses/Blueprints/EnumsAndStructs/WingDoorStructure` _array_element_2))
              (bind _returnvalue_9 (select `/Game/ModularMedievalHouses/Blueprints/EnumsAndStructs/ExtentionEnum` _extention_2 :`NewEnumerator0` (`self.LeftWing`) :`NewEnumerator1` (`self.RightWing`) :`NewEnumerator2` (`self.Extention1.0`) :`NewEnumerator3` (`self.Extention1.1`) :`NewEnumerator4` (`self.Extention2.0`) :`NewEnumerator5` (`self.Extention2.1`)))
              (bind _returnvalue_10 (`AddComponent|StaticMeshComponent_188` :`RelativeTransform` (`SceneComponent.GetSocketTransform` _returnvalue_9 (select `/Game/ModularMedievalHouses/Blueprints/EnumsAndStructs/WingEnum` _location_2 :`NewEnumerator0` "Window1" :`NewEnumerator1` "Window2" :`NewEnumerator2` "Window3" :`NewEnumerator3` "Window4" :`NewEnumerator4` "Window5" :`NewEnumerator5` "Window6" :!type "Name") "RTS_Actor")))
              (if (== (`SceneComponent.GetRelativeTransform` _returnvalue_10) (`SceneComponent.GetRelativeTransform` _returnvalue_9))
                (`ActorComponent.K2_DestroyComponent` _returnvalue_10)
                (else
                  (bind _returnvalue_11 (select `/Game/ModularMedievalHouses/Blueprints/EnumsAndStructs/DoorTypeEnum` _door :`NewEnumerator0` "/Game/ModularMedievalHouses/Meshes/SM_StoneFrameDoor.SM_StoneFrameDoor" :`NewEnumerator1` "/Game/ModularMedievalHouses/Meshes/SM_WoodframeDoor.SM_WoodframeDoor" :!type "StaticMesh Object Reference"))
                  (`KismetArrayLibrary.Array_Add` (`ActorComponent.ComponentTags` _returnvalue_10) (`KismetStringLibrary.Conv_StringToName` (`KismetStringLibrary.BuildString_Object` "" "" _returnvalue_11)))
                  (`StaticMeshComponent.SetStaticMesh` _returnvalue_10 _returnvalue_11))))))))
    (:`then_6`
      ;[1 1 1] Chimney
      (if (> _returnvalue_3 0)
        (for _index_3 (range _returnvalue_3)
          (bind _returnvalue_12 (`AddComponent|StaticMeshComponent_25` :`RelativeTransform` (`KismetArrayLibrary.Array_Get` (`.Location_8_6544D7254C424E9AB684BBBBD1E74D9C` (break `/Game/ModularMedievalHouses/Blueprints/EnumsAndStructs/ChimneyStructure` (`KismetArrayLibrary.Array_Get` _chimney _index_3))))))
          (`KismetArrayLibrary.Array_Add` (`ActorComponent.ComponentTags` _returnvalue_12) "Chimney")
          (`StaticMeshComponent.SetStaticMesh` _returnvalue_12 "/Game/ModularMedievalHouses/Meshes/SM_Chimney.SM_Chimney"))))
    (:`then_7`
      ;[1 1 1] Age
      (for _array_element_3 (`self.GetComponentsByTag` "/Script/Engine.StaticMeshComponent" "Building")
        (bind _returnvalue_13 (`PrimitiveComponent.CreateDynamicMaterialInstance` _array_element_3 0 "/Game/ModularMedievalHouses/Materials/StoneMaterial.StoneMaterial"))
        (`MaterialInstanceDynamic.SetScalarParameterValue` _returnvalue_13 "Age" _age)
        (bind _returnvalue_14 (`PrimitiveComponent.CreateDynamicMaterialInstance` _array_element_3 2 "/Game/ModularMedievalHouses/Materials/Instances/Wood_Inst1.Wood_Inst1"))
        (`MaterialInstanceDynamic.SetScalarParameterValue` _returnvalue_14 "Age" _age)
        (bind _returnvalue_15 (`PrimitiveComponent.CreateDynamicMaterialInstance` _array_element_3 3 "/Game/ModularMedievalHouses/Materials/Wall.Wall"))
        (`MaterialInstanceDynamic.SetScalarParameterValue` _returnvalue_15 "Age" _age)
        (bind _returnvalue_16 (`PrimitiveComponent.CreateDynamicMaterialInstance` _array_element_3 4 "/Game/ModularMedievalHouses/Materials/Wood.Wood"))
        (`MaterialInstanceDynamic.SetScalarParameterValue` _returnvalue_16 "Age" _age)
        (bind _returnvalue_17 (`PrimitiveComponent.CreateDynamicMaterialInstance` _array_element_3 5 "/Game/ModularMedievalHouses/Materials/Wall.Wall"))
        (`MaterialInstanceDynamic.SetScalarParameterValue` _returnvalue_17 "Age" _age)
        (bind _returnvalue_18 (`PrimitiveComponent.CreateDynamicMaterialInstance` _array_element_3 6 "/Game/ModularMedievalHouses/Materials/Instances/HouseRoofMaterialInstance.HouseRoofMaterialInstance"))
        (`MaterialInstanceDynamic.SetScalarParameterValue` _returnvalue_18 "Age" _age)
        (`MaterialInstanceDynamic.SetScalarParameterValue` _returnvalue_18 "Texture" (`KismetMathLibrary.Conv_IntToDouble` (`self.Texture`))))
      (for _array_element_4 (`self.GetComponentsByTag` "/Script/Engine.StaticMeshComponent" "Balcony")
        (bind _returnvalue_19 (`PrimitiveComponent.CreateDynamicMaterialInstance` _array_element_4 0 "/Game/ModularMedievalHouses/Materials/Planks.Planks"))
        (`MaterialInstanceDynamic.SetScalarParameterValue` _returnvalue_19 "Age" _age_4)
        (bind _returnvalue_20 (`PrimitiveComponent.CreateDynamicMaterialInstance` _array_element_4 1 "/Game/ModularMedievalHouses/Materials/Wood.Wood"))
        (`MaterialInstanceDynamic.SetScalarParameterValue` _returnvalue_20 "Age" _age_4)
        (bind _returnvalue_21 (`PrimitiveComponent.CreateDynamicMaterialInstance` _array_element_4 2 "/Game/ModularMedievalHouses/Materials/Wood.Wood"))
        (`MaterialInstanceDynamic.SetScalarParameterValue` _returnvalue_21 "Age" _age_4)
        (bind _returnvalue_22 (`PrimitiveComponent.CreateDynamicMaterialInstance` _array_element_4 3 "/Game/ModularMedievalHouses/Materials/Wood.Wood"))
        (`MaterialInstanceDynamic.SetScalarParameterValue` _returnvalue_22 "Age" _age_4))
      (for _array_element_5 (`self.GetComponentsByTag` "/Script/Engine.StaticMeshComponent" "SM_WoodFrameDoor")
        (bind _returnvalue_23 (`PrimitiveComponent.CreateDynamicMaterialInstance` _array_element_5 0 "/Game/ModularMedievalHouses/Materials/Wood.Wood"))
        (`MaterialInstanceDynamic.SetScalarParameterValue` _returnvalue_23 "Age" _age_3)
        (bind _returnvalue_24 (`PrimitiveComponent.CreateDynamicMaterialInstance` _array_element_5 1 "/Game/ModularMedievalHouses/Materials/DoorMaterial.DoorMaterial"))
        (`MaterialInstanceDynamic.SetScalarParameterValue` _returnvalue_24 "Age" _age_3))
      (for _array_element_6 (`self.GetComponentsByTag` "/Script/Engine.StaticMeshComponent" "Chimney")
        (bind _returnvalue_25 (`PrimitiveComponent.CreateDynamicMaterialInstance` _array_element_6 0 "/Game/ModularMedievalHouses/Materials/StoneMaterial2.StoneMaterial2"))
        (`MaterialInstanceDynamic.SetScalarParameterValue` _returnvalue_25 "Age" (`self.Age`)))
      (for _array_element_7 (`self.GetComponentsByTag` "/Script/Engine.StaticMeshComponent" "SM_StoneFrameDoor")
        (bind _returnvalue_26 (`PrimitiveComponent.CreateDynamicMaterialInstance` _array_element_7 0 "/Game/ModularMedievalHouses/Materials/StoneDoorMaterial.StoneDoorMaterial"))
        (`MaterialInstanceDynamic.SetScalarParameterValue` _returnvalue_26 "Age" _age_2)
        (bind _returnvalue_27 (`PrimitiveComponent.CreateDynamicMaterialInstance` _array_element_7 1 "/Game/ModularMedievalHouses/Materials/DoorMaterial.DoorMaterial"))
        (`MaterialInstanceDynamic.SetScalarParameterValue` _returnvalue_27 "Age" _age_2)))
    (:`then_8`
      ;[1 1 1] Collision
      (for _array_element_8 (`self.K2_GetComponentsByClass` "/Script/Engine.StaticMeshComponent")
        (`PrimitiveComponent.SetCollisionObjectType` _array_element_8 "ECC_WorldStatic")))
    (:`then_9`
      ;[1 1 1] Show Location
      (if (`self.Show Locations`)
        (for _array_element_9 (`SceneComponent.GetAllSocketNames` _staticmesh)
          (bind _returnvalue_28 (`AddComponent|Text Render Component_0` :`RelativeTransform` (`KismetMathLibrary.MakeTransform` (`KismetMathLibrary.MakeVector` (* (.x (.location (`SceneComponent.GetSocketTransform` _staticmesh _array_element_9 "RTS_Actor"))) 1.15) (* (.y (.location (`SceneComponent.GetSocketTransform` _staticmesh _array_element_9 "RTS_Actor"))) 1.15) (+ (.z (.location (`SceneComponent.GetSocketTransform` _staticmesh _array_element_9 "RTS_Actor"))) 100.0)) (`KismetMathLibrary.ComposeRotators` (.rotation (`SceneComponent.GetSocketTransform` _staticmesh _array_element_9 "RTS_Actor")) (struct :`Yaw` 90.0)) (.scale (`SceneComponent.GetSocketTransform` _staticmesh _array_element_9 "RTS_Actor")))))
          (`TextRenderComponent.K2_SetText` _returnvalue_28 (`KismetTextLibrary.Conv_NameToText` _array_element_9))
          (`TextRenderComponent.SetWorldSize` _returnvalue_28 40.0)
          (`TextRenderComponent.SetHorizontalAlignment` _returnvalue_28 "EHTA_Center"))))
    (:`then_10`
      ;[1 1 1] Show wing/extention location
      (if (`self.ShowWingLocations`)
        (bind _output_get (set `self.StaticMeshComponents` (`self.K2_GetComponentsByClass` "/Script/Engine.StaticMeshComponent")))
        (`KismetArrayLibrary.Array_RemoveItem` _output_get (`self.StaticMesh`))
        (for _array_element_10 (`self.StaticMeshComponents`)
          (bind _asstatic_mesh_component (cast `StaticMeshComponent` _array_element_10))
          (for _array_element_11 (`SceneComponent.GetAllSocketNames` _asstatic_mesh_component)
            (bind _returnvalue_29 (`AddComponent|TextRenderComponent_780` :`RelativeTransform` (`KismetMathLibrary.MakeTransform` (`KismetMathLibrary.MakeVector` (* (.x (.location (`SceneComponent.GetSocketTransform` _asstatic_mesh_component _array_element_11 "RTS_Actor"))) 1.15) (* (.y (.location (`SceneComponent.GetSocketTransform` _asstatic_mesh_component _array_element_11 "RTS_Actor"))) 1.15) (+ (.z (.location (`SceneComponent.GetSocketTransform` _asstatic_mesh_component _array_element_11 "RTS_Actor"))) 100.0)) (`KismetMathLibrary.ComposeRotators` (.rotation (`SceneComponent.GetSocketTransform` _asstatic_mesh_component _array_element_11 "RTS_Actor")) (struct :`Yaw` 90.0)) (.scale (`SceneComponent.GetSocketTransform` _asstatic_mesh_component _array_element_11 "RTS_Actor")))))
            (`TextRenderComponent.K2_SetText` _returnvalue_29 (`KismetTextLibrary.Conv_NameToText` _array_element_11))
            (`TextRenderComponent.SetWorldSize` _returnvalue_29 40.0)
            (`TextRenderComponent.SetHorizontalAlignment` _returnvalue_29 "EHTA_Center")))))))