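; Modular medieval tower that assembles itself in the construction script from editable arrays, with no gameplay logic.
; Stacks floor, railing or roof meshes at fixed height steps above the base mesh and places stone or wood framed doors at its window sockets.
; Tags each added piece by mesh name, then uses those tags to apply per-slot dynamic materials sharing an Age value, plus a roof Texture option.
; Finally sets every mesh to WorldStatic collision.
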(fn `UserConstructionScript`
  (bind _door (`self.Door`))
  (bind _towerstructure (`self.TowerStructure`))
  (bind _age (`self.Age`))
  (bind _age_2 (`self.Age`))
  (bind _age_3 (`self.Age`))
  (bind _age_4 (`self.Age`))
  (bind _age_5 (`self.Age`))
  (bind _staticmesh (`self.StaticMesh`))
  (bind _age_6 (`self.Age`))
  (bind _returnvalue (`KismetArrayLibrary.Array_Length` _towerstructure))
  (bind _returnvalue_2 (`KismetArrayLibrary.Array_Length` _door))
  (`|ExecutionSequence`
    (:`then_0`
      ;[1 1 1] Comment
      (if (> _returnvalue 0)
        (for _index (range _returnvalue)
          (bind _returnvalue_3 (`AddComponent|StaticMeshComponent_9` :`RelativeTransform` (`KismetMathLibrary.MakeTransform` (* (0.0 0.0 277.0) (+ _index 1)))))
          (bind _returnvalue_4 (select `/Game/ModularMedievalHouses/Blueprints/EnumsAndStructs/TowerEnum` (`.StaticMesh_8_E6821B5849A6D5C4BB94149EBD095CEA` (break `/Game/ModularMedievalHouses/Blueprints/EnumsAndStructs/TowerStructure` (`KismetArrayLibrary.Array_Get` _towerstructure _index))) :`NewEnumerator0` "/Game/ModularMedievalHouses/Meshes/SM_TowerFloor.SM_TowerFloor" :`NewEnumerator1` "/Game/ModularMedievalHouses/Meshes/SM_TowerRailing.SM_TowerRailing" :`NewEnumerator2` "/Game/ModularMedievalHouses/Meshes/SM_TowerRoof.SM_TowerRoof" :!type "StaticMesh Object Reference"))
          (`KismetArrayLibrary.Array_Add` (`ActorComponent.ComponentTags` _returnvalue_3) (`KismetStringLibrary.Conv_StringToName` (`KismetStringLibrary.BuildString_Object` "" "" _returnvalue_4)))
          (`StaticMeshComponent.SetStaticMesh` _returnvalue_3 _returnvalue_4))))
    (:`then_1`
      ;[1 1 1] Door
      (if (> _returnvalue_2 0)
        (for _index_2 (range _returnvalue_2)
          (bind (_doortype _doorlocation) (break `/Game/ModularMedievalHouses/Blueprints/EnumsAndStructs/DoorStructureTower` (`KismetArrayLibrary.Array_Get` _door _index_2)))
          (bind _returnvalue_5 (`AddComponent|StaticMeshComponent_539` :`RelativeTransform` (`SceneComponent.GetSocketTransform` (`self.StaticMesh`) (select `/Game/ModularMedievalHouses/Blueprints/EnumsAndStructs/DoorEnumTower` _doorlocation :`NewEnumerator0` "Window1" :`NewEnumerator1` "Window2" :`NewEnumerator2` "Window3" :`NewEnumerator3` "Window4" :!type "Name") "RTS_Actor")))
          (bind _returnvalue_6 (select `/Game/ModularMedievalHouses/Blueprints/EnumsAndStructs/DoorTypeEnum` _doortype :`NewEnumerator0` "/Game/ModularMedievalHouses/Meshes/SM_StoneFrameDoor.SM_StoneFrameDoor" :`NewEnumerator1` "/Game/ModularMedievalHouses/Meshes/SM_WoodframeDoor.SM_WoodframeDoor" :!type "StaticMesh Object Reference"))
          (`KismetArrayLibrary.Array_Add` (`ActorComponent.ComponentTags` _returnvalue_5) (`KismetStringLibrary.Conv_StringToName` (`KismetStringLibrary.BuildString_Object` "" "" _returnvalue_6)))
          (`StaticMeshComponent.SetStaticMesh` _returnvalue_5 _returnvalue_6))))
    (:`then_2`
      ;[1 1 1] Age
      (bind _returnvalue_7 (`PrimitiveComponent.CreateDynamicMaterialInstance` _staticmesh 0 "/Game/ModularMedievalHouses/Materials/StoneMaterial.StoneMaterial"))
      (`MaterialInstanceDynamic.SetScalarParameterValue` _returnvalue_7 "Age" _age_2)
      (bind _returnvalue_8 (`PrimitiveComponent.CreateDynamicMaterialInstance` _staticmesh 2 "/Game/ModularMedievalHouses/Materials/Instances/Wood_Inst1.Wood_Inst1"))
      (`MaterialInstanceDynamic.SetScalarParameterValue` _returnvalue_8 "Age" _age_2)
      (bind _returnvalue_9 (`PrimitiveComponent.CreateDynamicMaterialInstance` _staticmesh 3 "/Game/ModularMedievalHouses/Materials/Wall.Wall"))
      (`MaterialInstanceDynamic.SetScalarParameterValue` _returnvalue_9 "Age" _age_2)
      (bind _returnvalue_10 (`PrimitiveComponent.CreateDynamicMaterialInstance` _staticmesh 4 "/Game/ModularMedievalHouses/Materials/Wood.Wood"))
      (`MaterialInstanceDynamic.SetScalarParameterValue` _returnvalue_10 "Age" _age_2)
      (bind _returnvalue_11 (`PrimitiveComponent.CreateDynamicMaterialInstance` _staticmesh 5 "/Game/ModularMedievalHouses/Materials/Wall.Wall"))
      (`MaterialInstanceDynamic.SetScalarParameterValue` _returnvalue_11 "Age" _age_2)
      (for _array_element (`self.GetComponentsByTag` "/Script/Engine.StaticMeshComponent" "SM_TowerFloor")
        (bind _returnvalue_12 (`PrimitiveComponent.CreateDynamicMaterialInstance` _array_element 0 "/Game/ModularMedievalHouses/Materials/StoneMaterial.StoneMaterial"))
        (`MaterialInstanceDynamic.SetScalarParameterValue` _returnvalue_12 "Age" _age_6)
        (bind _returnvalue_13 (`PrimitiveComponent.CreateDynamicMaterialInstance` _array_element 2 "/Game/ModularMedievalHouses/Materials/Instances/Wood_Inst1.Wood_Inst1"))
        (`MaterialInstanceDynamic.SetScalarParameterValue` _returnvalue_13 "Age" _age_6)
        (bind _returnvalue_14 (`PrimitiveComponent.CreateDynamicMaterialInstance` _array_element 3 "/Game/ModularMedievalHouses/Materials/Wall.Wall"))
        (`MaterialInstanceDynamic.SetScalarParameterValue` _returnvalue_14 "Age" _age_6)
        (bind _returnvalue_15 (`PrimitiveComponent.CreateDynamicMaterialInstance` _array_element 4 "/Game/ModularMedievalHouses/Materials/Wood.Wood"))
        (`MaterialInstanceDynamic.SetScalarParameterValue` _returnvalue_15 "Age" _age_6)
        (bind _returnvalue_16 (`PrimitiveComponent.CreateDynamicMaterialInstance` _array_element 5 "/Game/ModularMedievalHouses/Materials/Wall.Wall"))
        (`MaterialInstanceDynamic.SetScalarParameterValue` _returnvalue_16 "Age" _age_6))
      (for _array_element_2 (`self.GetComponentsByTag` "/Script/Engine.StaticMeshComponent" "SM_WoodFrameDoor")
        (bind _returnvalue_17 (`PrimitiveComponent.CreateDynamicMaterialInstance` _array_element_2 0 "/Game/ModularMedievalHouses/Materials/Wood.Wood"))
        (`MaterialInstanceDynamic.SetScalarParameterValue` _returnvalue_17 "Age" _age_3)
        (bind _returnvalue_18 (`PrimitiveComponent.CreateDynamicMaterialInstance` _array_element_2 1 "/Game/ModularMedievalHouses/Materials/DoorMaterial.DoorMaterial"))
        (`MaterialInstanceDynamic.SetScalarParameterValue` _returnvalue_18 "Age" _age_3))
      (for _array_element_3 (`self.GetComponentsByTag` "/Script/Engine.StaticMeshComponent" "SM_TowerRailing")
        (bind _returnvalue_19 (`PrimitiveComponent.CreateDynamicMaterialInstance` _array_element_3 0 "/Game/ModularMedievalHouses/Materials/Wood.Wood"))
        (`MaterialInstanceDynamic.SetScalarParameterValue` _returnvalue_19 "Age" _age)
        (bind _returnvalue_20 (`PrimitiveComponent.CreateDynamicMaterialInstance` _array_element_3 1 "/Game/ModularMedievalHouses/Materials/Wood.Wood"))
        (`MaterialInstanceDynamic.SetScalarParameterValue` _returnvalue_20 "Age" _age))
      (for _array_element_4 (`self.GetComponentsByTag` "/Script/Engine.StaticMeshComponent" "SM_StoneFrameDoor")
        (bind _returnvalue_21 (`PrimitiveComponent.CreateDynamicMaterialInstance` _array_element_4 0 "/Game/ModularMedievalHouses/Materials/StoneDoorMaterial.StoneDoorMaterial"))
        (`MaterialInstanceDynamic.SetScalarParameterValue` _returnvalue_21 "Age" _age_5)
        (bind _returnvalue_22 (`PrimitiveComponent.CreateDynamicMaterialInstance` _array_element_4 1 "/Game/ModularMedievalHouses/Materials/DoorMaterial.DoorMaterial"))
        (`MaterialInstanceDynamic.SetScalarParameterValue` _returnvalue_22 "Age" _age_5))
      (for _array_element_5 (`self.GetComponentsByTag` "/Script/Engine.StaticMeshComponent" "SM_TowerRoof")
        (bind _returnvalue_23 (`PrimitiveComponent.CreateDynamicMaterialInstance` _array_element_5 0 "/Game/ModularMedievalHouses/Materials/Wood.Wood"))
        (`MaterialInstanceDynamic.SetScalarParameterValue` _returnvalue_23 "Age" _age_4)
        (bind _returnvalue_24 (`PrimitiveComponent.CreateDynamicMaterialInstance` _array_element_5 1 "/Game/ModularMedievalHouses/Materials/Instances/TowerRoofMaterialInstance.TowerRoofMaterialInstance"))
        (`MaterialInstanceDynamic.SetScalarParameterValue` _returnvalue_24 "Age" _age_4)
        (`MaterialInstanceDynamic.SetScalarParameterValue` _returnvalue_24 "Texture" (`KismetMathLibrary.Conv_IntToDouble` (`self.Texture`)))
        (bind _returnvalue_25 (`PrimitiveComponent.CreateDynamicMaterialInstance` _array_element_5 2 "/Game/ModularMedievalHouses/Materials/Wood.Wood"))
        (`MaterialInstanceDynamic.SetScalarParameterValue` _returnvalue_25 "Age" _age_4)))
    (:`then_3`
      ;[1 1 1] Collision
      (for _array_element_6 (`self.K2_GetComponentsByClass` "/Script/Engine.StaticMeshComponent")
        (`PrimitiveComponent.SetCollisionObjectType` _array_element_6 "ECC_WorldStatic")))))